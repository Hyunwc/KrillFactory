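; BP_LampSwiitch is a clickable switch actor that toggles lamps in the level.
; When its MouseInteractComponent fires OnClicked, it prints a debug string, gathers all actors carrying its LightTag, casts each to BP_Lamp and calls ToggleOnOff.
; Linking switch to lamps by actor tag avoids direct references to individual lamps.
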(event OnClicked(MouseInteractComponent)
  (params (TouchedComponent :type Primitive%20Component%20Object%20Reference) (ButtonPressed :type Key%20Structure :default "None"))
  (Development|PrintString "CLick!")
  (bind _outactors (Actor|GetAllActorswithTag (Variables|Default|GetLightTag)))
  (for _array_element _outactors
    (bind _asbp_lamp (Utilities|Casting|CastToBP_Lamp _array_element))
    (Default|ToggleonOff _asbp_lamp)))

(event EventBeginPlay
  (|CallParentFunction) ; This node is disabled and will not be called.\nDrag off pins to build functionality.
)

(event Collision|EventActorBeginOverlap
  (params (OtherActor :type Actor%20Object%20Reference))
  (|CallParentFunction OtherActor) ; This node is disabled and will not be called.\nDrag off pins to build functionality.
)

(event EventTick
  (params (DeltaSeconds :type Float%20%28single-precision%29))
  (|CallParentFunction DeltaSeconds) ; This node is disabled and will not be called.\nDrag off pins to build functionality.
)

(fn ConstructionScript
  (|CallParentFunction))