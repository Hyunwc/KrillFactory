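; BP_PaintBucket is a paint bucket object that responds to the mouse cursor hovering over it.
; Its MouseInteractComponent cursor-over events begin and end focus on its InteractComponent.
; The Blueprint adds no other logic: BeginPlay, overlap and Tick are disabled stubs, and the construction script only calls its parent.
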(event OnBeginCursorOver(MouseInteractComponent)
  (params (TouchedComponent :type Primitive%20Component%20Object%20Reference))
  (Class|KFObjectInteractComponent|BeginFocus (Variables|Default|GetInteractComponent)))

(event OnEndCursorOver(MouseInteractComponent)
  (params (TouchedComponent :type Primitive%20Component%20Object%20Reference))
  (Class|KFObjectInteractComponent|EndFocus (Variables|Default|GetInteractComponent)))

(event EventBeginPlay
  (|CallParentFunction) ; This node is disabled and will not be called.\nDrag off pins to build functionality.
)

(event Collision|EventActorBeginOverlap
  (params (OtherActor :type Actor%20Object%20Reference))
  (|CallParentFunction OtherActor) ; This node is disabled and will not be called.\nDrag off pins to build functionality.
)

(event EventTick
  (params (DeltaSeconds :type Float%20%28single-precision%29))
  (|CallParentFunction DeltaSeconds) ; This node is disabled and will not be called.\nDrag off pins to build functionality.
)

(fn ConstructionScript
  (|CallParentFunction))