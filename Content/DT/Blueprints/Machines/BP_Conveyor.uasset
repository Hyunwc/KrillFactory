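; BP_Conveyor is a conveyor machine Blueprint whose graph handles only mouse-hover focus, with no belt or transport logic.
; MouseInteractComponent's cursor begin and end events call BeginFocus and EndFocus on InteractComponent.
; Logic to rotate PopupWidget toward the player camera is present but disconnected, so it never runs, and Tick is empty.
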(event OnBeginCursorOver(MouseInteractComponent)
  (params (TouchedComponent :type Primitive%20Component%20Object%20Reference))
  (Class|KFInteractComponent|BeginFocus (Variables|Default|GetInteractComponent)))

(event OnEndCursorOver(MouseInteractComponent)
  (params (TouchedComponent :type Primitive%20Component%20Object%20Reference))
  (Class|KFInteractComponent|EndFocus (Variables|Default|GetInteractComponent)))

(event EventBeginPlay)

(event Collision|EventActorBeginOverlap
  (params (OtherActor :type Actor%20Object%20Reference)))

(event EventTick
  (params (DeltaSeconds :type Float%20%28single-precision%29))
  ;[0 0 0 0.5] 위젯이 카메라를 바라보게 하는 로직
)

(fn ConstructionScript)