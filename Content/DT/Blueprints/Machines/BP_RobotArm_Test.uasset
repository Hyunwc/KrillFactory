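; Test robot arm machine actor that drives a skeletal mesh arm through the "joint2_ctrl" Control Rig control in world space.
; Tick sets that control to TestTrans every frame and prints a debug string.
; MoveArmtoTarget plays a timeline that writes the same control, lerping from the live GripSocket transform, re-sampled each update, toward the given target.
; The TestArm function and construction script are empty.
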(event EventBeginPlay)

(event Collision|EventActorBeginOverlap
  (params (OtherActor :type Actor%20Object%20Reference)))

(event EventTick
  (params (DeltaSeconds :type Float%20%28single-precision%29))
  (Class|ControlRigComponent|SetControlTransform (Variables|Default|GetControlRig) "joint2_ctrl" (Variables|Default|GetTestTrans) "WorldSpace")
  (Development|PrintString "여기 들어오네 ㅎㅎ"))

(event EventMoveArmtoTarget
  (params (Target :type Transform%20%28by%20ref%29))
  (bind _alpha (Timeline|MoveArmTimeLine PlayFromStart)
    (:Update
      (Class|ControlRigComponent|SetControlTransform (Variables|Default|GetControlRig) "joint2_ctrl" (Math|Transform|Lerp(Transform) (Transformation|GetSocketTransform (Variables|Default|GetSkeletalMesh) "GripSocket" "RTS_World") Target _alpha) "WorldSpace")
      (Development|PrintString "여기 들어오네 ㅎㅎ"))))

(fn ConstructionScript)

(fn TestArm)